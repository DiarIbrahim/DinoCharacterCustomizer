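; BP_Customizer is the pawn for character customization, applying appearances built from DA_CharacterDataBase.
; On BeginPlay it applies a minimal appearance, then opens W_CustomizationWidget bound to itself with game-and-UI input and a visible cursor.
; Space applies a random appearance from the database.
; Ctrl+2 saves the current appearance to a fixed slot on disk, and Ctrl+3 loads and applies it, each printing a confirmation.
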(event `self.ReceiveBeginPlay`
  (bind _returnvalue (`GameplayStatics.GetPlayerController` 0))
  (`|ExecutionSequence`
    (:`then_0`
      (bind _returnvalue_2 (`DinoCharacterCustomizerHelper.GenerateMinimalCharacterAppearanceFromDataBase` "/DinoCharacterCustomizer/DataBase/DA_CharacterDataBase.DA_CharacterDataBase"))
      (`self.ApplyCharacterAppearance` _returnvalue_2))
    (:`then_1`
      (bind _returnvalue_3 (`|CreateWidget` "/DinoCharacterCustomizer/Widgets/W_CustomizationWidget.W_CustomizationWidget_C" null self))
      (`UserWidget.AddToViewport` _returnvalue_3 0)
      (`WidgetBlueprintLibrary.SetInputMode_GameAndUIEx` _returnvalue _returnvalue_3)
      (set `PlayerController.bShowMouseCursor` true _returnvalue))))

(event `Key|SpaceBar`
  (params (Key :type "Key Structure"))
  (:`Pressed`
    (bind _returnvalue (`DinoCharacterCustomizerHelper.GenerateRandomCharacterAppearanceFromDatabase` "/DinoCharacterCustomizer/DataBase/DA_CharacterDataBase.DA_CharacterDataBase"))
    (`self.ApplyCharacterAppearance` _returnvalue)))

(event `Key|Ctrl+Two`
  (params (Key :type "Key Structure"))
  (:`Pressed`
    (`DinoCharacterCustomizerSaveGameHelper.SaveCharacterAppearance` (`self.GetCharacterAppearance`))
    (`KismetSystemLibrary.PrintString` "Appearance Saved to Disk")))

(event `Key|Ctrl+Three`
  (params (Key :type "Key Structure"))
  (:`Pressed`
    (bind _returnvalue (`DinoCharacterCustomizerSaveGameHelper.LoadCharacterAppearance` 0))
    (`self.ApplyCharacterAppearance` _returnvalue)
    (`KismetSystemLibrary.PrintString` "Appearance Loaded From Disk")))

(fn `UserConstructionScript`)