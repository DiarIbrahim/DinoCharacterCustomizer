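; BP_CustomizerStudio is a character customization studio that lets the player edit, save, load and randomize an appearance.
; On BeginPlay it initializes from the DDB_Charracter database with minimal appearance, then opens W_CustomizationWidget with mouse input, or prints a failure.
; Hotkeys save and load appearance slot 1 or apply a random appearance generated from the database, debug-printing each result.
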(event `self.ReceiveBeginPlay`
  (bind _returnvalue (`GameplayStatics.GetPlayerController` 0))
  (bind _returnvalue_2 (`self.InitializeCustomizationFromDatabase` "/DinoCustomizer/DataBase/DDB_Charracter.DDB_Charracter"))
  (if _returnvalue_2
    (bind _returnvalue_3 (`|CreateWidget` "/DinoCustomizer/Widgets/W_CustomizationWidget.W_CustomizationWidget_C" null self))
    (`UserWidget.AddToViewport` _returnvalue_3 0)
    (`WidgetBlueprintLibrary.SetInputMode_GameAndUIEx` _returnvalue null)
    (set `PlayerController.bShowMouseCursor` true _returnvalue)
    (else
      (`KismetSystemLibrary.PrintText` "---------- Failed Init"))))

(event `Key|Ctrl+Two`
  (params (Key :type "Key Structure"))
  (bind _returnvalue (`self.GetCustomizationAppearance`))
  (:`Pressed`
    (`DinoCharacterCustomizerSaveGameHelper.SaveCustomizationAppearance` _returnvalue 1)
    (`DinoCustomizerHelper.DebugPrintAppearance` _returnvalue 10.0 (struct :`R` 1.0 :`G` 0.250452 :`A` 1.0))))

(event `Key|Ctrl+Three`
  (params (Key :type "Key Structure"))
  (:`Pressed`
    (bind _returnvalue (`DinoCharacterCustomizerSaveGameHelper.LoadCustomizationAppearance` 1))
    (`self.ApplyCustomizationAppearance` _returnvalue)
    (`DinoCustomizerHelper.DebugPrintAppearance` _returnvalue 10.0 (struct :`G` 0.113013 :`B` 1.0 :`A` 1.0))))

(event `Key|SpaceBar`
  (params (Key :type "Key Structure"))
  (:`Pressed`
    (bind _returnvalue (`DinoCustomizerHelper.GenerateRandomCustomizationAppearanceFromDatabase` "/DinoCustomizer/DataBase/DDB_Charracter.DDB_Charracter"))
    (`DinoCustomizerHelper.DebugPrintAppearance` _returnvalue 10.0 (struct :`R` 1.0 :`B` 0.894343 :`A` 1.0))
    (`self.ApplyCustomizationAppearance` _returnvalue)))

(fn `UserConstructionScript`)